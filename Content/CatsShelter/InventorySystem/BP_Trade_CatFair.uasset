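; Cat fair trade actor where the player sells highbred cats, highlighted through custom depth stencil on overlap.
; It opens a WBP_CatFair showcase to move cats between the player's inventory and fair slots, pricing them by age, fleas and worms.
; Participating pays out the total, removes matching cats from the game instance, skips time through BP_TimeSystem and updates the highbred tutorial quest.
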(event EventBeginOverlap
  (bind _staticmesh (Variables|Default|GetStaticMesh))
  (Rendering|SetRenderCustomDepth _staticmesh true)
  (Rendering|SetCustomDepthStencilValue _staticmesh 2))

(event EventEndOverlap
  (bind _staticmesh (Variables|Default|GetStaticMesh))
  (Rendering|SetRenderCustomDepth _staticmesh false)
  (Rendering|SetCustomDepthStencilValue _staticmesh 0))

(fn ConstructionScript
  (|CallParentFunction))

(fn OpenShowcase
  (|CallParentFunction)
  (bind _widgetofshowcase (Variables|Default|GetWidgetOfShowcase)
    (:then
      (bind _aswbp_cat_fair (Utilities|Casting|CastToWBP_CatFair _widgetofshowcase))
      (bind _output_get (Variables|Default|SetCatFairShowcase _aswbp_cat_fair))
      (Variables|/Game/CatsShelter/UI/Shops/WBP_CatFair.WBP_CatFair_C|SetCatFairShop _output_get self)
      (Variables|/Game/CatsShelter/UI/Shops/WBP_CatFair.WBP_CatFair_C|SetCatFairInventory _output_get (Variables|Default|GetBP_InventoryComponent_Trade))
      (bind _asthird_person_character (Utilities|Casting|CastToThirdPersonCharacter (Game|GetPlayerCharacter 0)))
      (Variables|/Game/CatsShelter/UI/Shops/WBP_CatFair.WBP_CatFair_C|SetCharacterInventory (Variables|Default|GetCatFairShowcase) (Variables|/Game/CatsShelter/Core/MainCharacter/ThirdPersonCharacter.ThirdPersonCharacter_C|GetInventory _asthird_person_character))
      (UserInterface|Viewport|AddtoViewport (Variables|Default|GetCatFairShowcase) 0)
      (return))
    (:else
      (return))))

(fn ChooseCat
  (params (ChosenSlotIndex :type Integer))
  (if (== (Variables|Default|GetChosenCat) -1)
    (Variables|Default|SetChosenCat ChosenSlotIndex)
    (return true)
    (elif (== ChosenSlotIndex (Variables|Default|GetChosenCat))
      (Variables|Default|SetChosenCat -1)
      (return false)
      (else
        (bind _array_element (Utilities|Array|ForEachLoopwithBreak (Class|PanelWidget|GetAllChildren (Variables|/Game/CatsShelter/UI/Shops/WBP_Showcase_ChooseCat.WBP_Showcase_ChooseCat_C|GetGridOfCats (Variables|/Game/CatsShelter/UI/Shops/WBP_CatFair.WBP_CatFair_C|GetWBP_Showcase_ChooseCat (Variables|Default|GetCatFairShowcase)))) :!label _label)
          (:LoopBody
            (bind _aswbp_cat_slot (Utilities|Casting|CastToWBP_CatSlot _array_element))
            (if (== (Variables|/Game/CatsShelter/UI/Shops/WBP_CatSlot.WBP_CatSlot_C|GetSlotID _aswbp_cat_slot) (Variables|Default|GetChosenCat))
              (LocalVariables|SetCatSlotTemp _aswbp_cat_slot)
              (goto _label Break)))
          (:Completed
            (Default|SetSlotNotChosen (LocalVariables|GetCatSlotTemp))
            (Variables|Default|SetChosenCat ChosenSlotIndex)
            (return true)))))))

(fn SetCatinThisSlot
  (params (ChosenEmptySlotID :type Integer))
  (bind (_choosencatinfo _isanycatchoosen) (CallFunction|GetChosenCatInfo))
  (if _isanycatchoosen
    (if (== (Variables|/Game/CatsShelter/Blueprints/Cats/CatInfo.CatInfo_C|GetCatType _choosencatinfo) "/Game/CatsShelter/Blueprints/Cats/HighbredCat.HighbredCat_C")
      (bind _output_get (LocalVariables|SetCatForSetInfo _choosencatinfo))
      (bind _price (CallFunction|GetCatPrice _output_get))
      (bind _output_get_2 (Variables|/Game/CatsShelter/Blueprints/Cats/CatInfo.CatInfo_C|SetPrice _output_get _price))
      (Utilities|Array|SetArrayElem (Variables|/Game/CatsShelter/InventorySystem/BP_InventoryComponent.BP_InventoryComponent_C|GetList%20of%20Slots (Variables|Default|GetBP_InventoryComponent_Trade)) ChosenEmptySlotID (Utilities|Struct|MakeSInventorySlot (Utilities|Struct|MakeSInventoryItem (Variables|/Game/CatsShelter/Blueprints/Cats/CatInfo.CatInfo_C|GetName _output_get) "/Game/CatsShelter/Blueprints/Widgets/smilingCat.smilingCat" false 100 1.0 "/Game/CatsShelter/InventorySystem/BP_InventoryItem_Cat.BP_InventoryItem_Cat_C" _output_get _output_get_2) 1 1.0))
      (Default|SetCatFairInventory (Variables|Default|GetCatFairShowcase))
      (CallFunction|DeleteChosenCatfromCharacter)
      (Variables|Default|SetChosenCat -1)
      (return true)
      (else
        (bind _asthird_person_game_mode (Utilities|Casting|CastToThirdPersonGameMode (Game|GetGameMode)))
        (Default|ShowNotification _asthird_person_game_mode "You can't sell a not highbred cat!" 1e+01)
        (return false)))
    (else
      (bind _asthird_person_game_mode_2 (Utilities|Casting|CastToThirdPersonGameMode (Game|GetGameMode)))
      (Default|ShowNotification _asthird_person_game_mode_2 "Choose a cat!" 1e+01)
      (return false))))

(fn GetChosenCatInfo
  (if (!= (Variables|Default|GetChosenCat) -1)
    (bind _array_element (Utilities|Array|ForEachLoopwithBreak (Class|PanelWidget|GetAllChildren (Variables|/Game/CatsShelter/UI/Shops/WBP_Showcase_ChooseCat.WBP_Showcase_ChooseCat_C|GetGridOfCats (Variables|/Game/CatsShelter/UI/Shops/WBP_CatFair.WBP_CatFair_C|GetWBP_Showcase_ChooseCat (Variables|Default|GetCatFairShowcase)))) :!label _label)
      (:LoopBody
        (bind _aswbp_cat_slot (Utilities|Casting|CastToWBP_CatSlot _array_element))
        (if (== (Variables|/Game/CatsShelter/UI/Shops/WBP_CatSlot.WBP_CatSlot_C|GetSlotID _aswbp_cat_slot) (Variables|Default|GetChosenCat))
          (LocalVariables|SetChosenCatInfotemp (Variables|/Game/CatsShelter/UI/Shops/WBP_CatSlot.WBP_CatSlot_C|GetCatInfo _aswbp_cat_slot))
          (LocalVariables|SetCatID (Variables|/Game/CatsShelter/UI/Shops/WBP_CatSlot.WBP_CatSlot_C|GetCatIDInPlayerInventory _aswbp_cat_slot))
          (goto _label Break)))
      (:Completed
        (return (LocalVariables|GetChosenCatInfotemp) true (LocalVariables|GetCatID))))
    (else
      (return 0 false -1))))

(fn DeleteChosenCatfromCharacter
  (bind (_choosencatinfo _isanycatchoosen _catidincharacterinventory) (CallFunction|GetChosenCatInfo))
  (if _isanycatchoosen
    (bind _asthird_person_character (Utilities|Casting|CastToThirdPersonCharacter (Game|GetPlayerCharacter 0)))
    (Default|DeletefromInventory (Variables|/Game/CatsShelter/Core/MainCharacter/ThirdPersonCharacter.ThirdPersonCharacter_C|GetInventory _asthird_person_character) _catidincharacterinventory 1.0)
    (Default|SetCatsTakenbyPlayer (Variables|Default|GetCatFairShowcase))
    (return)))

(fn ReturnCattoInventory
  (params (ChoosenSlotID :type Integer) (CatInfo :type Cat%20Info%20Object%20Reference))
  (bind _catfairshowcase (Variables|Default|GetCatFairShowcase))
  (bind _asthird_person_character (Utilities|Casting|CastToThirdPersonCharacter (Game|GetPlayerCharacter 0)))
  (bind _output_get (LocalVariables|SetPlayerInventory (Variables|/Game/CatsShelter/Core/MainCharacter/ThirdPersonCharacter.ThirdPersonCharacter_C|GetInventory _asthird_person_character)))
  (bind _succeed (Default|AddItemtoInventory _output_get (Utilities|Struct|MakeSInventoryItem "_PH" "/Game/CatsShelter/Blueprints/Widgets/smilingCat.smilingCat" false 100 1.0 "/Game/CatsShelter/InventorySystem/BP_InventoryItem_Cat.BP_InventoryItem_Cat_C" CatInfo)))
  (if _succeed
    (Utilities|Array|SetArrayElem (Variables|/Game/CatsShelter/InventorySystem/BP_InventoryComponent.BP_InventoryComponent_C|GetList%20of%20Slots (Variables|Default|GetBP_InventoryComponent_Trade)) ChoosenSlotID (Utilities|Struct|MakeSInventorySlot (Utilities|Struct|MakeSInventoryItem "_PH" "/Game/CatsShelter/Core/MainCharacter/Mannequin/Character/Textures/UE4_LOGO_CARD.UE4_LOGO_CARD") 1 1.0))
    (Default|SetCatFairInventory _catfairshowcase)
    (Default|SetCatsTakenbyPlayer _catfairshowcase)
    (return true)
    (else
      (bind _asthird_person_game_mode (Utilities|Casting|CastToThirdPersonGameMode (Game|GetGameMode)))
      (Default|ShowNotification _asthird_person_game_mode "You have no space in the inventory!" 1e+01)
      (return false))))

(fn ParticipateinFair
  (for (_array_element _array_index) (Variables|/Game/CatsShelter/InventorySystem/BP_InventoryComponent.BP_InventoryComponent_C|GetList%20of%20Slots (Variables|Default|GetBP_InventoryComponent_Trade))
    (if (== (.class (.itemstructure _array_element)) "/Game/CatsShelter/InventorySystem/BP_InventoryItem_Cat.BP_InventoryItem_Cat_C")
      (LocalVariables|SetTotalIncome (+ (Variables|/Game/CatsShelter/Blueprints/Cats/CatInfo.CatInfo_C|GetPrice (.catinfo (.itemstructure _array_element))) (LocalVariables|GetTotalIncome)))
      (bind _asbp_main_game_instance (Utilities|Casting|CastToBP_MainGameInstance (Game|GetGameInstance)))
      (bind (_array_element_2 _array_index_2) (Utilities|Array|ForEachLoopwithBreak (Variables|/Game/CatsShelter/Core/BP_MainGameInstance.BP_MainGameInstance_C|GetCats _asbp_main_game_instance) :!label _label)
        (:LoopBody
          (if (Math|Boolean|ANDBoolean (== (Variables|/Game/CatsShelter/Blueprints/Cats/CatInfo.CatInfo_C|GetUrineNeedInPercent _array_element_2) (Variables|/Game/CatsShelter/Blueprints/Cats/CatInfo.CatInfo_C|GetUrineNeedInPercent (.catinfo (.itemstructure _array_element)))) (Utilities|Enum|Equal(Enum) (Variables|/Game/CatsShelter/Blueprints/Cats/CatInfo.CatInfo_C|GetName _array_element_2) (Variables|/Game/CatsShelter/Blueprints/Cats/CatInfo.CatInfo_C|GetName (.catinfo (.itemstructure _array_element)))) (== (Variables|/Game/CatsShelter/Blueprints/Cats/CatInfo.CatInfo_C|GetAge _array_element_2) (Variables|/Game/CatsShelter/Blueprints/Cats/CatInfo.CatInfo_C|GetAge (.catinfo (.itemstructure _array_element)))) (Math|Boolean|Equal(Boolean) (Variables|/Game/CatsShelter/Blueprints/Cats/CatInfo.CatInfo_C|GetisFemale _array_element_2) (Variables|/Game/CatsShelter/Blueprints/Cats/CatInfo.CatInfo_C|GetisFemale (.catinfo (.itemstructure _array_element)))) (== (Variables|/Game/CatsShelter/Blueprints/Cats/CatInfo.CatInfo_C|GetCatType _array_element_2) (Variables|/Game/CatsShelter/Blueprints/Cats/CatInfo.CatInfo_C|GetCatType (.catinfo (.itemstructure _array_element)))))
            (Utilities|Array|RemoveIndex (Variables|/Game/CatsShelter/Core/BP_MainGameInstance.BP_MainGameInstance_C|GetCats _asbp_main_game_instance) _array_index_2)
            (goto _label Break)))
        (:Completed
          (Utilities|Array|SetArrayElem (Variables|/Game/CatsShelter/InventorySystem/BP_InventoryComponent.BP_InventoryComponent_C|GetList%20of%20Slots (Variables|Default|GetBP_InventoryComponent_Trade)) _array_index (Utilities|Struct|MakeSInventorySlot (Utilities|Struct|MakeSInventoryItem "_PH" "/Game/CatsShelter/Core/MainCharacter/Mannequin/Character/Textures/UE4_LOGO_CARD.UE4_LOGO_CARD") 1 1.0))))))
  (Default|GetIncome (Variables|Default|GetBP_InventoryComponent_Trade) (LocalVariables|GetTotalIncome))
  (Default|SetCatFairInventory (Variables|Default|GetCatFairShowcase))
  (bind _returnvalue (Actor|GetActorOfClass "/Game/CatsShelter/Core/BP_TimeSystem.BP_TimeSystem_C"))
  (Default|SkipPartOfDay _returnvalue (Variables|Default|GetDurationOfTheFair) (LocalVariables|GetSpeedOfSkipping))
  (bind _asthird_person_game_mode (Utilities|Casting|CastToThirdPersonGameMode (Game|GetGameMode)))
  (Default|UpdateQuest _asthird_person_game_mode "/Game/CatsShelter/Quests/Tutorial/BP_Tutorial_Highbred.BP_Tutorial_Highbred_C" 1)
  (return))

(fn GetCatPrice
  (params (CatInfo :type Cat%20Info%20Object%20Reference))
  (Utilities|FlowControl|Sequence
    (:then_0
      (if (Variables|/Game/CatsShelter/Blueprints/Cats/CatInfo.CatInfo_C|GethasFleas CatInfo)
        (Math|Integer|IncrementInt (LocalVariables|GetnumOfDesease))))
    (:then_1
      (if (Variables|/Game/CatsShelter/Blueprints/Cats/CatInfo.CatInfo_C|GethasWorms CatInfo)
        (Math|Integer|IncrementInt (LocalVariables|GetnumOfDesease))))
    (:then_2
      (bind _output_get (LocalVariables|SetretPrice (/ (- 2000 (Math|Float|Truncate (* (Math|Float|Sqrt (Math|Float|Power (Math|Conversions|ToFloat(Integer) (- (Variables|/Game/CatsShelter/Blueprints/Cats/CatInfo.CatInfo_C|GetAge CatInfo) 4)) 2.0)) 5e+02))) (+ (LocalVariables|GetnumOfDesease) 1))))
      (if (< _output_get 300)
        (LocalVariables|SetretPrice 300)
        (elif (> _output_get 5000)
          (LocalVariables|SetretPrice 5000))))
    (:then_3
      (return (LocalVariables|GetretPrice)))))