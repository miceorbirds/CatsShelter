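; BP_Trade_Petshop is the pet shop trade actor of the inventory system, extending a parent trade Blueprint.
; On overlap it toggles custom depth and stencil on its static mesh, marking it while something is in range.
; Its OpenShowcase override runs the parent logic, casts the showcase widget to WBP_Petshop, hands it the trade inventory component and adds it to the viewport.
; A SetInputMode node is left unconnected.
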(event EventBeginOverlap
  (bind _staticmesh (Variables|Default|GetStaticMesh))
  (Rendering|SetRenderCustomDepth _staticmesh true)
  (Rendering|SetCustomDepthStencilValue _staticmesh 2))

(event EventEndOverlap
  (bind _staticmesh (Variables|Default|GetStaticMesh))
  (Rendering|SetRenderCustomDepth _staticmesh false)
  (Rendering|SetCustomDepthStencilValue _staticmesh 0))

(fn ConstructionScript
  (|CallParentFunction))

(fn OpenShowcase
  (|CallParentFunction)
  (bind _widgetofshowcase (Variables|Default|GetWidgetOfShowcase)
    (:then
      (bind _aswbp_petshop (Utilities|Casting|CastToWBP_Petshop _widgetofshowcase))
      (Variables|/Game/CatsShelter/UI/Shops/WBP_Petshop.WBP_Petshop_C|SetShopInventory _aswbp_petshop (Variables|Default|GetBP_InventoryComponent_Trade))
      (bind _output_get (Variables|Default|SetPetshopShowcase _aswbp_petshop))
      (UserInterface|Viewport|AddtoViewport _output_get 0)
      (return))
    (:else
      (return))))