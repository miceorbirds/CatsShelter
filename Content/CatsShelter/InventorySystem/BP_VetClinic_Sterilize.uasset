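; Vet clinic sterilization item for the cat shelter inventory system, applied to a cat through UseItem.
; If the cat is not yet sterilized, it sets the flag, advances the sterilization tutorial quest and shows a notification via ThirdPersonGameMode.
; It then returns success with the updated cat in a new item struct that has placeholder name and thumbnail.
; An already sterilized cat only triggers a notice and returns failure.
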(event EventBeginPlay)

(event Collision|EventActorBeginOverlap
  (params (OtherActor :type Actor%20Object%20Reference)))

(event EventTick
  (params (DeltaSeconds :type Float%20%28single-precision%29)))

(fn ConstructionScript
  (|CallParentFunction))

(fn UseItem
  (params (ItemInfo :type S%20Inventory%20Item%20Structure))
  (bind _output_get (LocalVariables|SetTreatedCat (.CatInfo (Utilities|Struct|BreakSInventoryItem ItemInfo))))
  (if (not (Variables|/Game/CatsShelter/Blueprints/Cats/CatInfo.CatInfo_C|GetisSterilized _output_get))
    (Variables|/Game/CatsShelter/Blueprints/Cats/CatInfo.CatInfo_C|SetisSterilized (LocalVariables|GetTreatedCat) true)
    (bind _asthird_person_game_mode (Utilities|Casting|CastToThirdPersonGameMode (Game|GetGameMode)))
    (Default|UpdateQuest _asthird_person_game_mode "/Game/CatsShelter/Quests/Tutorial/BP_Tutorial_Sterilize.BP_Tutorial_Sterilize_C" 1)
    (Default|ShowNotification _asthird_person_game_mode (Utilities|Text|ToText(String) (Utilities|String|Append (Utilities|String|ToString(Text) (Variables|/Game/CatsShelter/Blueprints/Cats/CatInfo.CatInfo_C|GetName (LocalVariables|GetTreatedCat))) " has sterilized")) 1e+01)
    (return (Utilities|Struct|MakeSInventoryItem "_PH" "/Game/CatsShelter/Core/MainCharacter/Mannequin/Character/Textures/UE4_LOGO_CARD.UE4_LOGO_CARD" false 100 1.0 0 (LocalVariables|GetTreatedCat)) true)
    (else
      (bind _asthird_person_game_mode_2 (Utilities|Casting|CastToThirdPersonGameMode (Game|GetGameMode)))
      (Default|ShowNotification _asthird_person_game_mode_2 "Cat is sterilized already" 1e+01)
      (return "" false))))