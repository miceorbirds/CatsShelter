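; BP_VetClinic_Antiworms is a vet clinic antiworm item that cures worms on a cat carried in inventory item info.
; UseItem reads the cat data, clears HasWorms if set, prints a Russian confirmation and returns success with a rebuilt inventory item.
; The rebuilt item keeps the updated cat but uses a placeholder name and thumbnail.
; A cat without worms triggers a message and a failure result.
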(event EventBeginPlay)

(event Collision|EventActorBeginOverlap
  (params (OtherActor :type Actor%20Object%20Reference)))

(event EventTick
  (params (DeltaSeconds :type Float%20%28single-precision%29)))

(fn ConstructionScript
  (|CallParentFunction))

(fn UseItem
  (params (ItemInfo :type S%20Inventory%20Item%20Structure))
  (bind _output_get (LocalVariables|SetTreatedCat (.CatInfo (Utilities|Struct|BreakSInventoryItem ItemInfo))))
  (if (Variables|/Game/CatsShelter/Blueprints/Cats/CatInfo.CatInfo_C|GethasWorms _output_get)
    (Variables|/Game/CatsShelter/Blueprints/Cats/CatInfo.CatInfo_C|SethasWorms (LocalVariables|GetTreatedCat) false)
    (Development|PrintString (Utilities|String|Append (Utilities|String|ToString(Text) (Variables|/Game/CatsShelter/Blueprints/Cats/CatInfo.CatInfo_C|GetName _output_get)) " полечили глисты!"))
    (return (Utilities|Struct|MakeSInventoryItem "_PH" "/Game/CatsShelter/Core/MainCharacter/Mannequin/Character/Textures/UE4_LOGO_CARD.UE4_LOGO_CARD" false 100 1.0 0 (LocalVariables|GetTreatedCat)) true)
    (else
      (Development|PrintString "У кота нет глистов")
      (return "" false))))