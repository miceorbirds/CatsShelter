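; BP_InventoryItem is an inventory item actor that can be picked up in the world.
; Interact passes its ItemContent to the interactor's BP_InventoryComponent and destroys the actor if the add succeeds.
; BeginOverlap and EndOverlap toggle custom depth and stencil on the item mesh to drive an outline highlight.
; UseItem is a stub that always reports failure.
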(event EventInteract
  (params (Interactor :type Actor%20Object%20Reference))
  ;[1 1 1] Interaction
  (bind _succeed (Default|AddItemtoInventory (Actor|GetComponentbyClass Interactor "/Game/CatsShelter/InventorySystem/BP_InventoryComponent.BP_InventoryComponent_C") (Variables|Default|GetItemContent)))
  (if _succeed
    (Actor|DestroyActor)))

(event EventBeginOverlap
  (bind _itemmesh (Variables|Default|GetItemMesh))
  ;[1 1 1] Outline
  (Rendering|SetRenderCustomDepth _itemmesh true)
  (Rendering|SetCustomDepthStencilValue _itemmesh 2))

(event EventEndOverlap
  (bind _itemmesh (Variables|Default|GetItemMesh))
  ;[1 1 1] Outline
  (Rendering|SetRenderCustomDepth _itemmesh false)
  (Rendering|SetCustomDepthStencilValue _itemmesh 0))

(fn ConstructionScript)

(fn UseItem
  (params (ItemInfo :type S%20Inventory%20Item%20Structure))
  (return "" false))