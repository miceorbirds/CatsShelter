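; Trade inventory component that holds a shop's item slots and handles the player's purchases.
; BuyItem checks money and space, adds the item to the player's BP_InventoryComponent, charges the price, then removes it from the shop slot.
; Money changes go through BP_MainGameInstance, and GetIncome also shows an income notification via ThirdPersonGameMode.
; Purchases of cat food or Antiwormer advance tutorial quests, matched by item name string.
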(fn DeletefromInventory
  (params (ItemIndex :type Integer) (AmountOfItem :type Float%20%28single-precision%29))
  (bind _output_get (LocalVariables|SetShowcaseSlotForUsing (Utilities|Array|Get(acopy) (Variables|Default|GetList%20of%20Slots) ItemIndex)))
  ;[1 1 1] If we have 0,0 amount of thing, we clean the slot
  (bind _output_get_2 (LocalVariables|SetNewAmountOfItem (- (.sumofportions _output_get) AmountOfItem)))
  (if (== _output_get_2 0.0)
    (LocalVariables|SetOutputShowcaseSlot (LocalVariables|GetShowcaseSlotForUsing))
    (bind _output_get_3 (LocalVariables|SetShowcaseSlotForUsing (Utilities|Struct|MakeSInventorySlot "(ItemName_20_DD63AEF84F10C5EA3A1BE98D8FC9F12D=NSLOCTEXT(\"[FBBB02994128C0953A2D4984A5D665C2]\", \"C422BA0E414913D0D08AB2AA93F55B08\", \"_PH\"),ItemThumbnail_21_69AFCAB44F430AD5A9E398AD538E3219=Texture2D'\"/Game/CatsShelter/Core/MainCharacter/Mannequin/Character/Textures/UE4_LOGO_CARD.UE4_LOGO_CARD\"',IsStackable_10_5E3A9CE144BD6296F8C57AA518B36B9B=False,MaxStackSize_13_B5B9EDC14F5295E5D45C249E60AFADF0=100,Portions_24_E4519AD3410F1B10D66C91AB608DA0F4=1.000000,Class_19_51932DC14BB274B64754209A0BEF413A=None,CatInfo_28_BF3AD0574C439846353FD1BEF8469768=None,Price_31_A5495A8E42D3AEF3A650779BE56C2763=0,Tip_34_999D22034DF9C6E567FEC88CFD085002=\"\")" 0 0.0)))
    (Utilities|Array|SetArrayElem (Variables|Default|GetList%20of%20Slots) ItemIndex _output_get_3)
    (else
      (bind _output_get_4 (LocalVariables|SetShowcaseSlotForUsing (Utilities|Struct|MakeSInventorySlot (.itemstructure (LocalVariables|GetShowcaseSlotForUsing)) (Math|Float|Ceil (/ (LocalVariables|GetNewAmountOfItem) (.portions (.itemstructure _output_get)))) (LocalVariables|GetNewAmountOfItem))))
      (Utilities|Array|SetArrayElem (Variables|Default|GetList%20of%20Slots) ItemIndex _output_get_4)
      (LocalVariables|SetShowcaseSlotForUsing (LocalVariables|GetShowcaseSlotForUsing))))
  (return (LocalVariables|GetOutputShowcaseSlot)))

(fn BuyItem
  (params (IndexOfSlot :type Integer))
  (bind _returnvalue (Game|Player|GetPlayerPawn 0))
  (bind _list_of_slots (Variables|Default|GetList%20of%20Slots))
  (bind _list_of_slots_2 (Variables|Default|GetList%20of%20Slots))
  (bind _returnvalue_2 (Actor|GetComponentbyClass _returnvalue "/Game/CatsShelter/InventorySystem/BP_InventoryComponent.BP_InventoryComponent_C"))
  (bind _output (Utilities|Array|Get(acopy) _list_of_slots IndexOfSlot))
  (bind _output_2 (Utilities|Array|Get(acopy) _list_of_slots_2 IndexOfSlot))
  (bind _itemstructure (Utilities|Struct|BreakSInventorySlot _output_2))
  (bind _enoughmoney (CallFunction|IsEnoughMoney (.Price (Utilities|Struct|BreakSInventoryItem _itemstructure))))
  (LocalVariables|SetEnoughMoney _enoughmoney)
  (bind _enoughspace (Default|CheckSpaceandStack _returnvalue_2 _itemstructure))
  (LocalVariables|SetEnoughSpace _enoughspace)
  (if (and (LocalVariables|GetEnoughMoney) (LocalVariables|GetEnoughSpace))
    (bind _succeed (Default|AddItemtoInventory _returnvalue_2 (.itemstructure _output)))
    (if _succeed
      (bind _sucsess (CallFunction|PaythePrice (.Price (Utilities|Struct|BreakSInventoryItem (.itemstructure _output)))))
      (if _sucsess
        (bind _inventoryslot (CallFunction|DeletefromInventory IndexOfSlot (.sumofportions _output)))
        (CallFunction|CheckBuyQuests _inventoryslot)
        (return true)
        (else
          _))))
  (return false))

(fn PaythePrice
  (params (Price :type Integer))
  (bind _asbp_main_game_instance (Utilities|Casting|CastToBP_MainGameInstance (Game|GetGameInstance)))
  (Default|UpdateMoney _asbp_main_game_instance Price true)
  (return true))

(fn IsEnoughMoney
  (params (Price :type Integer))
  (bind _asbp_main_game_instance (Utilities|Casting|CastToBP_MainGameInstance (Game|GetGameInstance)))
  (bind _isenough (Default|IsEnoughMoney _asbp_main_game_instance Price))
  (return _isenough))

(fn GetIncome
  (params (Income :type Integer))
  (bind _asbp_main_game_instance (Utilities|Casting|CastToBP_MainGameInstance (Game|GetGameInstance)))
  (Default|UpdateMoney _asbp_main_game_instance Income false)
  (bind _asthird_person_game_mode (Utilities|Casting|CastToThirdPersonGameMode (Game|GetGameMode)))
  (Default|ShowNotification _asthird_person_game_mode (Utilities|Text|ToText(String) (Utilities|String|BuildString(Integer) "" "Your income is " Income "!")) 1e+01)
  (return true))

(fn CheckBuyQuests
  (params (Slot :type S%20Inventory%20Slot%20Structure))
  (bind _itemstructure (Utilities|Struct|BreakSInventorySlot Slot))
  (bind _itemname (Utilities|Struct|BreakSInventoryItem _itemstructure))
  (bind _returnvalue (Utilities|String|ToString(Text) _itemname))
  (Utilities|FlowControl|Sequence
    (:then_0
      (if (or (Utilities|Enum|Equal(Enum) _returnvalue "Cat Food Premium") (Utilities|Enum|Equal(Enum) _returnvalue "Cat Food"))
        (bind _asthird_person_game_mode (Utilities|Casting|CastToThirdPersonGameMode (Game|GetGameMode)))
        (Default|UpdateQuest _asthird_person_game_mode "/Game/CatsShelter/Quests/Tutorial/BP_Tutorial_BuyKibble.BP_Tutorial_BuyKibble_C" 1)))
    (:then_1
      (if (Utilities|Enum|Equal(Enum) _returnvalue "Antiwormer")
        (bind _asthird_person_game_mode_2 (Utilities|Casting|CastToThirdPersonGameMode (Game|GetGameMode)))
        (Default|UpdateQuest _asthird_person_game_mode_2 "/Game/CatsShelter/Quests/Tutorial/BP_Tutorial_BuyPills.BP_Tutorial_BuyPills_C" 1)))))