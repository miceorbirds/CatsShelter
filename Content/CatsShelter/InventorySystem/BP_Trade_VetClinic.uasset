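; Vet clinic trade shop in a cat shelter game, where the player pays to treat a chosen cat, with a stencil outline toggled on overlap.
; OpenShowcase wires the WBP_VetClinic widget to the clinic and character inventories, while ChooseCat keeps a single selected slot.
; TreatTheCat checks selection and money, then spawns a temporary treatment actor to run UseItem, charging and updating the slot's CatInfo only on success.
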(event EventBeginOverlap
  (bind _staticmesh (Variables|Default|GetStaticMesh))
  (Rendering|SetRenderCustomDepth _staticmesh true)
  (Rendering|SetCustomDepthStencilValue _staticmesh 2))

(event EventEndOverlap
  (bind _staticmesh (Variables|Default|GetStaticMesh))
  (Rendering|SetRenderCustomDepth _staticmesh false)
  (Rendering|SetCustomDepthStencilValue _staticmesh 0))

(fn ConstructionScript
  (|CallParentFunction))

(fn OpenShowcase
  (|CallParentFunction)
  (bind _widgetofshowcase (Variables|Default|GetWidgetOfShowcase)
    (:then
      (bind _aswbp_vet_clinic (Utilities|Casting|CastToWBP_VetClinic _widgetofshowcase))
      (bind _output_get (Variables|Default|SetVetClinicShowcase _aswbp_vet_clinic))
      (Variables|/Game/CatsShelter/UI/Shops/WBP_VetClinic.WBP_VetClinic_C|SetVetClinicShop _output_get self)
      (Variables|/Game/CatsShelter/UI/Shops/WBP_VetClinic.WBP_VetClinic_C|SetVetClinicInventory _output_get (Variables|Default|GetBP_InventoryComponent_Trade))
      (bind _asthird_person_character (Utilities|Casting|CastToThirdPersonCharacter (Game|GetPlayerCharacter 0)))
      (Variables|/Game/CatsShelter/UI/Shops/WBP_VetClinic.WBP_VetClinic_C|SetCharacterInventory (Variables|Default|GetVetClinicShowcase) (Variables|/Game/CatsShelter/Core/MainCharacter/ThirdPersonCharacter.ThirdPersonCharacter_C|GetInventory _asthird_person_character))
      (UserInterface|Viewport|AddtoViewport (Variables|Default|GetVetClinicShowcase) 0)
      (return))
    (:else
      (Variables|Default|SetChosenCat -1)
      (return))))

(fn ChooseCat
  (params (ChosenSlotIndex :type Integer))
  (if (== (Variables|Default|GetChosenCat) -1)
    (Variables|Default|SetChosenCat ChosenSlotIndex)
    (return true)
    (elif (== ChosenSlotIndex (Variables|Default|GetChosenCat))
      (Variables|Default|SetChosenCat -1)
      (return false)
      (else
        (bind _array_element (Utilities|Array|ForEachLoopwithBreak (Class|PanelWidget|GetAllChildren (Variables|/Game/CatsShelter/UI/Shops/WBP_Showcase_ChooseCat.WBP_Showcase_ChooseCat_C|GetGridOfCats (Variables|/Game/CatsShelter/UI/Shops/WBP_VetClinic.WBP_VetClinic_C|GetWBP_Showcase_ChooseCat (Variables|Default|GetVetClinicShowcase)))) :!label _label)
          (:LoopBody
            (bind _aswbp_cat_slot (Utilities|Casting|CastToWBP_CatSlot _array_element))
            (if (== (Variables|/Game/CatsShelter/UI/Shops/WBP_CatSlot.WBP_CatSlot_C|GetSlotID _aswbp_cat_slot) (Variables|Default|GetChosenCat))
              (LocalVariables|SetCatSlotTemp _aswbp_cat_slot)
              (goto _label Break)))
          (:Completed
            (Default|SetSlotNotChosen (LocalVariables|GetCatSlotTemp))
            (Variables|Default|SetChosenCat ChosenSlotIndex)
            (return true)))))))

(fn GetChoosenCatInfo
  (if (!= (Variables|Default|GetChosenCat) -1)
    (bind _array_element (Utilities|Array|ForEachLoopwithBreak (Class|PanelWidget|GetAllChildren (Variables|/Game/CatsShelter/UI/Shops/WBP_Showcase_ChooseCat.WBP_Showcase_ChooseCat_C|GetGridOfCats (Variables|/Game/CatsShelter/UI/Shops/WBP_VetClinic.WBP_VetClinic_C|GetWBP_Showcase_ChooseCat (Variables|Default|GetVetClinicShowcase)))) :!label _label)
      (:LoopBody
        (bind _aswbp_cat_slot (Utilities|Casting|CastToWBP_CatSlot _array_element))
        (if (== (Variables|/Game/CatsShelter/UI/Shops/WBP_CatSlot.WBP_CatSlot_C|GetSlotID _aswbp_cat_slot) (Variables|Default|GetChosenCat))
          (LocalVariables|SetChoosenCatInfoTemp (Variables|/Game/CatsShelter/UI/Shops/WBP_CatSlot.WBP_CatSlot_C|GetCatInfo _aswbp_cat_slot))
          (goto _label Break)))
      (:Completed
        (return (LocalVariables|GetChoosenCatInfoTemp) true)))
    (else
      (return 0 false))))

(fn TreattheCat
  (params (treatmentType :type BP%20Inventory%20Item%20Class%20Reference) (Price :type Integer))
  (bind (_choosencatinfo _isanycatchoosen) (CallFunction|GetChoosenCatInfo))
  (if _isanycatchoosen
    (LocalVariables|SetInfoOfTreatedCat _choosencatinfo)
    (bind _enoughmoney (Default|IsEnoughMoney (Variables|Default|GetBP_InventoryComponent_Trade) Price))
    (if _enoughmoney
      (bind _returnvalue (Game|SpawnActorfromClass treatmentType (Math|Transform|MakeTransform "0, 0, 0") "DontSpawnIfColliding" 0 0))
      (bind _output_get (LocalVariables|SetTreatmentActorTemp _returnvalue))
      (bind (_changediteminfo _sucsess) (Default|UseItem _output_get (Utilities|Struct|MakeSInventoryItem "_PH" "/Game/CatsShelter/Core/MainCharacter/Mannequin/Character/Textures/UE4_LOGO_CARD.UE4_LOGO_CARD" false 100 1.0 0 (LocalVariables|GetInfoOfTreatedCat))))
      (if _sucsess
        (Default|PaythePrice (Variables|Default|GetBP_InventoryComponent_Trade) Price)
        (Actor|DestroyActor (LocalVariables|GetTreatmentActorTemp))
        (bind _sucsess_2 (CallFunction|SetChoosenCatInfo (.CatInfo (Utilities|Struct|BreakSInventoryItem _changediteminfo))))
        (return _sucsess_2)
        (else
          (Actor|DestroyActor (LocalVariables|GetTreatmentActorTemp))
          (return false)))
      (else
        (bind _asthird_person_game_mode (Utilities|Casting|CastToThirdPersonGameMode (Game|GetGameMode)))
        (Default|ShowNotification _asthird_person_game_mode "You have not enough money!" 1e+01)
        (return false)))
    (else
      (bind _asthird_person_game_mode_2 (Utilities|Casting|CastToThirdPersonGameMode (Game|GetGameMode)))
      (Default|ShowNotification _asthird_person_game_mode_2 "First of all chose the cat, that you want to treat!" 1e+01)
      (return false))))

(fn SetChoosenCatInfo
  (params (ChangedCatInfo :type Cat%20Info%20Object%20Reference))
  (if (!= (Variables|Default|GetChosenCat) -1)
    (bind _array_element (Utilities|Array|ForEachLoopwithBreak (Class|PanelWidget|GetAllChildren (Variables|/Game/CatsShelter/UI/Shops/WBP_Showcase_ChooseCat.WBP_Showcase_ChooseCat_C|GetGridOfCats (Variables|/Game/CatsShelter/UI/Shops/WBP_VetClinic.WBP_VetClinic_C|GetWBP_Showcase_ChooseCat (Variables|Default|GetVetClinicShowcase)))) :!label _label)
      (:LoopBody
        (bind _aswbp_cat_slot (Utilities|Casting|CastToWBP_CatSlot _array_element))
        (if (== (Variables|/Game/CatsShelter/UI/Shops/WBP_CatSlot.WBP_CatSlot_C|GetSlotID _aswbp_cat_slot) (Variables|Default|GetChosenCat))
          (Variables|/Game/CatsShelter/UI/Shops/WBP_CatSlot.WBP_CatSlot_C|SetCatInfo _aswbp_cat_slot ChangedCatInfo)
          (goto _label Break)))
      (:Completed
        (return true)))
    (else
      (return false))))