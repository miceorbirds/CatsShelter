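; BP_Trade is a shop actor that a ThirdPersonCharacter opens and closes by interacting.
; Its construction script fills BPInventoryComponentTrade from ItemsToSell, retrying each unit until the add succeeds, so a failed add can loop endlessly.
; OpenShowcase toggles the showcase widget, creating it without a visible viewport add, and ending overlap closes it.
; SetInputMode switches input and cursor by widget validity but is never called here.
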(event EventInteract
  (params (Interactor :type Actor%20Object%20Reference))
  ;[1 1 1] Open/close the shop
  (Utilities|Casting|CastToThirdPersonCharacter Interactor)
  (CallFunction|OpenShowcase))

(event Collision|EventActorEndOverlap
  (params (OtherActor :type Actor%20Object%20Reference))
  ;[1 1 1] Close the shop when run away
  (Variables|Default|GetWidgetOfShowcase
    (:then
      (CallFunction|OpenShowcase))
    (:else)))

(fn ConstructionScript
  (for _array_element (Variables|Default|GetItemsToSell)
    (bind _output_get (LocalVariables|SetAmountOfitem (.amount _array_element)))
    (while (> _output_get 0)
      (bind _succeed (Default|AddItemtoInventory (Variables|Default|GetBP_InventoryComponent_Trade) (Utilities|GetClassDefaults (.itemforsell _array_element))))
      (if _succeed
        (LocalVariables|SetAmountOfitem (- (LocalVariables|GetAmountOfitem) 1))))))

(fn OpenShowcase
  (bind _widgetofshowcase (Variables|Default|GetWidgetOfShowcase)
    (:then
      (Widget|RemovefromParent _widgetofshowcase)
      (Variables|Default|SetWidgetOfShowcase 0))
    (:else
      (bind _returnvalue (UserInterface|CreateWidget (Variables|Default|GetTypeOfWidget)))
      (Variables|Default|SetWidgetOfShowcase _returnvalue)))
  (return))

(fn SetInputMode
  (bind _returnvalue (Game|GetPlayerController 0))
  (bind _widgetofshowcase (Variables|Default|GetWidgetOfShowcase)
    (:then
      (Input|SetInputModeGameandUI _returnvalue _widgetofshowcase "LockAlways" true)
      (Variables|/Script/Engine.PlayerController|SetbShowMouseCursor _returnvalue true))
    (:else
      (Input|SetInputModeGameOnly _returnvalue)
      (Variables|/Script/Engine.PlayerController|SetbShowMouseCursor _returnvalue false)))
  (return))