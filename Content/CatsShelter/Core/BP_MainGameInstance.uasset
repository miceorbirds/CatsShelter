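; Game instance for a cat shelter game that holds the player's money, karma, active quest and cat records across the game.
; Money, quest and karma changes are pushed straight to MainUI widgets, and karma caps at 100 while dropping to zero pauses and shows the endgame menu.
; It creates CatInfo objects and checks given-away cats against BP_TimeSystem hours, asking the game mode for one overdue adoption result per call.
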(event Custom|FreedomCat
  (Variables|Default|SetFreeCat true))

(event EventInit)

(fn CreateCatInfo
  (bind _returnvalue (Game|ConstructObjectfromClass "/Game/CatsShelter/Blueprints/Cats/CatInfo.CatInfo_C" self))
  (Utilities|Array|Add (Variables|Default|GetCats) _returnvalue)
  (return _returnvalue))

(fn UpdateMoney
  (params (Amount :type Integer) (DoWeBuy :type Boolean))
  (if DoWeBuy
    (Variables|Default|SetMoney (- (Variables|Default|GetMoney) Amount))
    (else
      (Variables|Default|SetMoney (+ (Variables|Default|GetMoney) Amount))))
  (Variables|/Game/CatsShelter/UI/WBP_MainUI.WBP_MainUI_C|SetMoney (Variables|Default|GetMainUI) (Variables|Default|GetMoney))
  (return))

(fn IsEnoughMoney
  (params (Price :type Integer))
  (if (>= (Variables|Default|GetMoney) Price)
    (return true)
    (else
      (return false))))

(fn UpdateTimeOfGivenCats
  (params (TimeToGiveAnswer :type Float%20%28single-precision%29))
  (bind _givencats (Variables|Default|GetGivenCats))
  (bind _returnvalue (Actor|GetActorOfClass "/Game/CatsShelter/Core/BP_TimeSystem.BP_TimeSystem_C"))
  (bind _values (Utilities|Map|Values _givencats))
  (bind (_array_element _array_index) (Utilities|Array|ForEachLoopwithBreak _values :!label _label)
    (:LoopBody
      (if (> (- (Math|Timespan|GetTotalHours (Variables|/Game/CatsShelter/Core/BP_TimeSystem.BP_TimeSystem_C|GetTimeOfDay _returnvalue)) _array_element) TimeToGiveAnswer)
        (bind _keys (Utilities|Map|Keys _givencats))
        (bind _asthird_person_game_mode (Utilities|Casting|CastToThirdPersonGameMode (Game|GetGameMode)))
        (Default|GetResultOfGiveAwayCat _asthird_person_game_mode (Utilities|Array|Get(acopy) _keys _array_index))
        (goto _label Break)))))

(fn SetQuest
  (params (Quest :type BP%20Quest%20Object%20Reference))
  (bind _mainui (Variables|Default|GetMainUI))
  (bind _wbp_quest (Variables|/Game/CatsShelter/UI/WBP_MainUI.WBP_MainUI_C|GetWBP_Quest _mainui))
  (Utilities|IsValid Quest
    (:Is%20Valid
      (bind _done (Default|IsDone Quest))
      (if _done
        (Variables|Default|SetQuest 0 :!label _label)
        (Variables|/Game/CatsShelter/UI/WBP_Quest.WBP_Quest_C|SetQuest _wbp_quest 0)
        (Widget|SetVisibility _wbp_quest "Hidden")
        (else
          (bind _output_get (Variables|Default|SetQuest Quest))
          (Variables|/Game/CatsShelter/UI/WBP_Quest.WBP_Quest_C|SetQuest _wbp_quest _output_get)
          (Widget|SetVisibility _wbp_quest "Visible"))))
    (:Is%20Not%20Valid
      (goto _label))))

(fn GetQuest
  (bind _quest (Variables|Default|GetQuest)
    (:then
      (bind _done (Default|IsDone _quest))
      (return _quest _done))
    (:else
      (return 0 false))))

(fn IncreaseKarma
  (params (Amount :type Integer))
  (bind _output_get (LocalVariables|SetNewKarma (+ Amount (Variables|Default|GetKarmaRate))))
  (if (> _output_get 100)
    (Variables|Default|SetKarmaRate 100)
    (else
      (Variables|Default|SetKarmaRate (LocalVariables|GetNewKarma))))
  (CallFunction|UpdateKarmaWidget))

(fn ReduceKarma
  (params (Amount :type Integer))
  (bind _output_get (LocalVariables|SetNewKarma (- (Variables|Default|GetKarmaRate) Amount)))
  (if (<= _output_get 0)
    (Game|SetGamePaused true)
    (bind _returnvalue (UserInterface|CreateWidget "/Game/CatsShelter/UI/WBP_MainMenu_Endgame.WBP_MainMenu_Endgame_C"))
    (UserInterface|Viewport|AddtoViewport _returnvalue 100)
    (else
      (Variables|Default|SetKarmaRate (LocalVariables|GetNewKarma))
      (CallFunction|UpdateKarmaWidget)
      (return))))

(fn UpdateKarmaWidget
  (Variables|/Game/CatsShelter/UI/WBP_KarmaRate.WBP_KarmaRate_C|SetKarmaAmount (Variables|/Game/CatsShelter/UI/WBP_MainUI.WBP_MainUI_C|GetWBP_KarmaRate (Variables|Default|GetMainUI)) (Variables|Default|GetKarmaRate)))