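; Day/night cycle actor that tracks game time and drives the sun, skylight and sky sphere.
; The SunMovement timeline, rate-scaled by DaySpeed, supplies sun rotation, light intensities and seconds, which Tick applies and converts to day, hour and minute for the main UI.
; BeginPlay restores saved time from the game instance; each timeline finish increments the day, calls the game mode's EverydayUpdate and restarts.
; SkipPartOfDay jumps the timeline by a timespan.
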(event EventBeginPlay
  (bind _asthird_person_game_mode (Utilities|Casting|CastToThirdPersonGameMode (Game|GetGameMode)))
  (Variables|Default|SetGameMode _asthird_person_game_mode)
  ;[1 1 1] Get desired time from the game instance
  (bind _asbp_main_game_instance (Utilities|Casting|CastToBP_MainGameInstance (Game|GetGameInstance))
    (:then
      (CallFunction|SetCurrentDayTime (Variables|/Game/CatsShelter/Core/BP_MainGameInstance.BP_MainGameInstance_C|GetCurrentTimeOfDay _asbp_main_game_instance))
      (bind (_direction _ysunpitch _zsunyaw _timeinseconds _skylightintensity _directionallightintensity) (Timeline|Sun%20Movement SetNewTime)
        (:Finished
          (CallFunction|DayCounter)
          (Timeline|Sun%20Movement PlayFromStart))))
    (:CastFailed
      (Timeline|Sun%20Movement SetNewTime))))

(event EventTick
  (params (DeltaSeconds :type Float%20%28single-precision%29))
  (CallFunction|ConvertSunMovementtoHoursandMin)
  (Variables|Default|SetTimeOfSunMovementInSec (stale EventBeginPlay _timeinseconds))
  (Transformation|SetActorRotation (Variables|Default|GetDirectionalLight) (Math|Rotator|MakeRotator 0.5 (stale EventBeginPlay _ysunpitch) (stale EventBeginPlay _zsunyaw)))
  (Rendering|Components|Light|SetIntensity (Variables|/Script/Engine.SkyLight|GetLightComponent (Variables|Default|GetSkyLight)) (stale EventBeginPlay _skylightintensity))
  (Rendering|Components|Light|SetIntensity (Variables|/Script/Engine.Light|GetLightComponent (Variables|Default|GetDirectionalLight)) (stale EventBeginPlay _directionallightintensity))
  (Default|UpdateSunDirection (Variables|Default|GetSkySphere))
  (CallFunction|DisplayTime))

(fn ConstructionScript
  (Utilities|FlowControl|Sequence
    (:then_0
      (Components|Timeline|SetPlayRate (Variables|Default|GetSun%20Movement) (Variables|Default|GetDaySpeed)))
    (:then_1
      (bind _returnvalue (Actor|GetActorOfClass "/Script/Engine.DirectionalLight"))
      (Variables|Default|SetDirectionalLight _returnvalue))
    (:then_2
      (bind _returnvalue_2 (Actor|GetActorOfClass "/Engine/EngineSky/BP_Sky_Sphere.BP_Sky_Sphere_C"))
      (Variables|Default|SetSkySphere _returnvalue_2))
    (:then_3
      (bind _returnvalue_3 (Actor|GetActorOfClass "/Script/Engine.SkyLight"))
      (Variables|Default|SetSkyLight _returnvalue_3))))

(fn ConvertSunMovementtoHoursandMin
  (Variables|Default|SetTimeOfDay (Math|Timespan|MakeTimespan (Variables|Default|GetCountOfDays) 0 0 (Math|Float|Truncate (Variables|Default|GetTimeOfSunMovementInSec)))))

(fn DayCounter
  (Variables|Default|SetCountOfDays (+ (Variables|Default|GetCountOfDays) 1))
  (Default|EverydayUpdate (Variables|Default|GetGameMode))
  (return))

(fn DisplayTime
  (bind _timeofday (Variables|Default|GetTimeOfDay))
  (bind _gamemode (Variables|Default|GetGameMode))
  (bind _mainui (Variables|/Game/CatsShelter/Core/ThirdPersonGameMode.ThirdPersonGameMode_C|GetMainUI _gamemode))
  (Variables|/Game/CatsShelter/UI/WBP_MainUI.WBP_MainUI_C|SetDays _mainui (Utilities|Text|ToText(Integer) (.days _timeofday)))
  (Variables|/Game/CatsShelter/UI/WBP_MainUI.WBP_MainUI_C|SetHours _mainui (Utilities|Text|ToText(Integer) (.hours _timeofday) false true 2))
  (Variables|/Game/CatsShelter/UI/WBP_MainUI.WBP_MainUI_C|SetMinutes _mainui (Utilities|Text|ToText(Integer) (.minutes _timeofday) false true 2)))

(fn SetCurrentDayTime
  (params (Time :type Timespan%20Structure))
  (Variables|Default|SetCountOfDays (.days Time))
  (Variables|Default|SetStartTime (CallFunction|TimeMath (.hours Time) (.minutes Time) (.seconds Time)))
  (return))

(fn TimeMath
  (params (Hours :type Integer) (Minutes :type Integer) (Seconds :type Integer))
  (return (+ (Math|Conversions|ToFloat(Integer) Hours) (/ (+ (Math|Conversions|ToFloat(Integer) Minutes) (/ (Math|Conversions|ToFloat(Integer) Seconds) 6e+01)) 6e+01))))

(fn SkipPartOfDay
  (params (Time :type Timespan%20Structure) (SpeedOfSkipping :type Float%20%28single-precision%29))
  (bind _timeofday (Variables|Default|GetTimeOfDay))
  (bind _returnvalue (+ Time _timeofday))
  (Components|Timeline|SetNewTime (Variables|Default|GetSun%20Movement) (CallFunction|TimeMath (.hours _returnvalue) (.minutes _returnvalue) (.seconds _returnvalue)))
  (return))