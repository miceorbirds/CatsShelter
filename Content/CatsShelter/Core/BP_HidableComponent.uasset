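; Actor component that fades its owner's static meshes in and out through material opacity.
; On BeginPlay it creates dynamic instances of every material on those meshes and stores them in one array.
; Hide and Show set mutually exclusive flags that Tick reads to step each Opacity parameter by delta time times fader speed.
; Each fade stops once the last material processed reaches fully transparent or opaque.
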(event EventBeginPlay
  ;[1 1 1] Get all materials of the owner for future hide/show work
  (for _array_element (Actor|GetComponentsByClass (Components|GetOwner) "/Script/Engine.StaticMeshComponent")
    (bind _output_get (Variables|Default|SetOwner'sStaticMesh _array_element))
    (for _index (range 0 (- (Utilities|Array|Length (Rendering|Material|GetMaterials _output_get)) 1))
      (bind _returnvalue (Rendering|Material|CreateDynamicMaterialInstance (Variables|Default|GetOwner'sStaticMesh) _index (Rendering|Material|GetMaterial (Variables|Default|GetOwner'sStaticMesh) _index) "None" :!class /Script/Engine.PrimitiveComponent))
      (Utilities|Array|Insert (Variables|Default|GetDynamicMaterials) _returnvalue _index)))
  (Development|PrintString "Dynamic materials created successfully"))

(event EventTick
  (params (DeltaSeconds :type Float%20%28single-precision%29))
  (bind _shouldhide_ (Variables|Default|GetShouldHide?))
  (if _shouldhide_
    (CallFunction|UpdateVisibility (* DeltaSeconds (Variables|Default|GetFaderSpeed)) _shouldhide_ :!label _label)
    (elif (Variables|Default|GetShouldShow?)
      (goto _label))))

(fn UpdateVisibility
  (params (Amount :type Float%20%28single-precision%29) (ShouldHide? :type Boolean))
  (if ShouldHide?
    (for _array_element (Variables|Default|GetDynamicMaterials)
      (bind _returnvalue (Rendering|Material|GetScalarParameterValue _array_element "Opacity" :!class /Script/Engine.MaterialInstanceDynamic))
      (bind _output_get (LocalVariables|SetLastAmountOfFadeWhenHide (- _returnvalue Amount)))
      (Rendering|Material|SetScalarParameterValue _array_element "Opacity" _output_get :!class /Script/Engine.MaterialInstanceDynamic))
    (Variables|Default|SetShouldHide? (not (<= (LocalVariables|GetLastAmountOfFadeWhenHide) 0.0)))
    (else
      (for _array_element_2 (Variables|Default|GetDynamicMaterials)
        (bind _returnvalue_2 (Rendering|Material|GetScalarParameterValue _array_element_2 "Opacity" :!class /Script/Engine.MaterialInstanceDynamic))
        (bind _output_get_2 (LocalVariables|SetLastAmountOfFadeWhenShow (+ _returnvalue_2 Amount)))
        (Rendering|Material|SetScalarParameterValue _array_element_2 "Opacity" _output_get_2 :!class /Script/Engine.MaterialInstanceDynamic))
      (Variables|Default|SetShouldShow? (not (>= (LocalVariables|GetLastAmountOfFadeWhenShow) 1.0)))))
  (return))

(fn Show
  (Variables|Default|SetShouldShow? true)
  (Variables|Default|SetShouldHide? false)
  (return))

(fn Hide
  (Variables|Default|SetShouldHide? true)
  (Variables|Default|SetShouldShow? false)
  (return))