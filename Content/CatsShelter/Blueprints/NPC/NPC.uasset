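; NPC townsperson in the cat shelter game that players can offer cats to for adoption.
; On BeginPlay it picks a random human skeletal mesh and rolls a 50% chance of wanting a cat.
; Interact checks the player's current inventory slot: a wanted cat goes through the game mode, updates the tutorial quest and is consumed; otherwise a greeting or refusal notification shows.
; Overlap events signal the player walking nearby or away.
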(event EventBeginPlay
  (CallFunction|SetRandomMesh)
  (Variables|Default|SetNeedCat (Math|Random|RandomBoolwithWeight 0.5)))

(event Collision|EventActorBeginOverlap
  (params (OtherActor :type Actor%20Object%20Reference)))

(event EventTick
  (params (DeltaSeconds :type Float%20%28single-precision%29)))

(event EventBeginOverlap
  (Default|CallPlayerWalkNearby))

(event EventEndOverlap
  (Default|CallPlayerWalkAway))

(event EventInteract
  (params (Interactor :type Actor%20Object%20Reference))
  (bind _asthird_person_character (Utilities|Casting|CastToThirdPersonCharacter Interactor))
  (if (== (.Class (Utilities|Struct|BreakSInventoryItem (.ItemStructure (Utilities|Struct|BreakSInventorySlot (Utilities|Array|Get(acopy) (Variables|/Game/CatsShelter/InventorySystem/BP_InventoryComponent.BP_InventoryComponent_C|GetList%20of%20Slots (Variables|/Game/CatsShelter/Core/MainCharacter/ThirdPersonCharacter.ThirdPersonCharacter_C|GetInventory _asthird_person_character)) (Variables|/Game/CatsShelter/InventorySystem/BP_InventoryComponent.BP_InventoryComponent_C|GetCurItem (Variables|/Game/CatsShelter/Core/MainCharacter/ThirdPersonCharacter.ThirdPersonCharacter_C|GetInventory _asthird_person_character))))))) "/Game/CatsShelter/InventorySystem/BP_InventoryItem_Cat.BP_InventoryItem_Cat_C")
    (if (Variables|Default|GetNeedCat)
      (bind _asthird_person_game_mode (Utilities|Casting|CastToThirdPersonGameMode (Game|GetGameMode)))
      (Default|GiveCat _asthird_person_game_mode (.CatInfo (Utilities|Struct|BreakSInventoryItem (.ItemStructure (Utilities|Struct|BreakSInventorySlot (Utilities|Array|Get(acopy) (Variables|/Game/CatsShelter/InventorySystem/BP_InventoryComponent.BP_InventoryComponent_C|GetList%20of%20Slots (Variables|/Game/CatsShelter/Core/MainCharacter/ThirdPersonCharacter.ThirdPersonCharacter_C|GetInventory _asthird_person_character)) (Variables|/Game/CatsShelter/InventorySystem/BP_InventoryComponent.BP_InventoryComponent_C|GetCurItem (Variables|/Game/CatsShelter/Core/MainCharacter/ThirdPersonCharacter.ThirdPersonCharacter_C|GetInventory _asthird_person_character))))))))
      (Default|UpdateQuest _asthird_person_game_mode "/Game/CatsShelter/Quests/Tutorial/BP_Tutorial_GiveCatToNPC.BP_Tutorial_GiveCatToNPC_C" 1)
      (Default|UseItem (Variables|/Game/CatsShelter/Core/MainCharacter/ThirdPersonCharacter.ThirdPersonCharacter_C|GetInventory _asthird_person_character) "/Game/CatsShelter/InventorySystem/BP_InventoryItem_Cat.BP_InventoryItem_Cat_C" 1.0)
      (Default|ShowNotification _asthird_person_game_mode "-Hello! I realy want a cat!" 1e+01)
      (Variables|Default|SetNeedCat false)
      (else
        (bind _asthird_person_game_mode_2 (Utilities|Casting|CastToThirdPersonGameMode (Game|GetGameMode)))
        (Default|ShowNotification _asthird_person_game_mode_2 "-Hello! Sorry, I don't need a cat(" 1e+01)))
    (else
      (bind _asthird_person_game_mode_3 (Utilities|Casting|CastToThirdPersonGameMode (Game|GetGameMode)))
      (Default|ShowNotification _asthird_person_game_mode_3 "-Hello! How are you?" 1e+01))))

(fn ConstructionScript)

(fn SetRandomMesh
  (bind _mesh (Variables|Character|GetMesh))
  (bind _mesh_2 (Variables|Character|GetMesh))
  (bind _mesh_3 (Variables|Character|GetMesh))
  (switch int (Math|Random|RandomIntegerinRange 0 6)
    (:0
      (Class|SkinnedMeshComponent|SetSkeletalMesh _mesh "/Game/CatsShelter/Assets/NPC/Female_Alternative.Female_Alternative" true))
    (:1
      (Class|SkinnedMeshComponent|SetSkeletalMesh _mesh "/Game/CatsShelter/Assets/NPC/Female_Casual.Female_Casual" true))
    (:2
      (Class|SkinnedMeshComponent|SetSkeletalMesh _mesh_2 "/Game/CatsShelter/Assets/NPC/Female_Dress.Female_Dress" true))
    (:3
      (Class|SkinnedMeshComponent|SetSkeletalMesh _mesh_2 "/Game/CatsShelter/Assets/NPC/Female_TankTop.Female_TankTop" true))
    (:4
      (Class|SkinnedMeshComponent|SetSkeletalMesh _mesh_3 "/Game/CatsShelter/Assets/NPC/Male_Casual.Male_Casual" true))
    (:5
      (Class|SkinnedMeshComponent|SetSkeletalMesh _mesh_3 "/Game/CatsShelter/Assets/NPC/Male_LongSleeve.Male_LongSleeve" true))
    (:6
      (Class|SkinnedMeshComponent|SetSkeletalMesh _mesh_3 "/Game/CatsShelter/Assets/NPC/Male_Suit.Male_Suit" true))))