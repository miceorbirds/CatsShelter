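; AI controller that wanders a shelter NPC around the level and makes it face the player who comes near.
; It loops AIMoveTo toward random "NPC_Point" TargetPoints roughly aligned on X or Y, accumulated in an uncleared array, falling back to random nearby points.
; NPC proximity events halt movement and turn its yaw toward the player via a timeline.
; Wandering resumes shortly after the player leaves or after a timeout.
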(event Custom|PlayerWalkedNearby_Event_0
  (bind _npc (Variables|Default|GetNPC))
  (bind _returnvalue (Transformation|GetActorRotation _npc))
  (Variables|Default|SetFreeToMove false)
  (AI|Navigation|StopMovement)
  (bind _alpha (Timeline|Timeline_0 PlayFromStart)
    (:Update
      (Transformation|SetActorRotation _npc (Math|Rotator|MakeRotator (.roll _returnvalue) (.pitch _returnvalue) (Math|Float|Lerp (.yaw _returnvalue) (.yaw (Math|Rotator|FindLookatRotation (Transformation|GetActorLocation _npc) (Transformation|GetActorLocation (Game|GetPlayerCharacter 0)))) _alpha))))
    (:Finished
      (Utilities|FlowControl|Delay 25.0)
      (CallFunction|PlayerWalkedAwayEvent0))))

(event Custom|GoToNextPoint
  (bind _npc (Variables|Default|GetNPC))
  (bind _returnvalue (Transformation|GetActorLocation _npc))
  (if (Variables|Default|GetFreeToMove)
    (bind (_properpoint _result) (CallFunction|GetProperTargetPoint _returnvalue))
    (if _result
      (AI|AIMoveTo _npc "0, 0, 0" _properpoint 5.0 false
        (:OnSuccess
          _)
        (:OnFail
          _))
      (CallFunction|GotoNextPoint)
      (else
        (AI|AIMoveTo (Variables|Default|GetNPC) (.RandomLocation (AI|Navigation|GetRandomReachablePointinRadius _returnvalue 3e+02 0 0)) 0 5.0 false
          (:OnSuccess
            _)
          (:OnFail
            _))
        (CallFunction|GotoNextPoint)))))

(event Custom|PlayerWalkedAway_Event_0
  (Utilities|FlowControl|Delay 2.0)
  (Variables|Default|SetFreeToMove true)
  (CallFunction|GotoNextPoint))

(event EventBeginPlay
  (bind _asnpc (Utilities|Casting|CastToNPC (Pawn|GetControlledPawn)))
  (bind _output_get (Variables|Default|SetNPC _asnpc))
  (CallFunction|GotoNextPoint)
  (EventDispatchers|BindEventtoPlayerWalkNearby _output_get (delegate Custom|PlayerWalkedNearby_Event_0))
  (EventDispatchers|BindEventtoPlayerWalkAway (Variables|Default|GetNPC) (delegate Custom|PlayerWalkedAway_Event_0)))

(event EventTick
  (params (DeltaSeconds :type Float%20%28single-precision%29)))

(fn ConstructionScript)

(fn GetProperTargetPoint
  (params (Location :type Vector))
  (bind _propertarget (LocalVariables|GetProperTarget))
  (bind _returnvalue (Utilities|Array|Length _propertarget))
  (bind _outactors (Actor|GetAllActorsOfClasswithTag "/Script/Engine.TargetPoint" "NPC_Point"))
  (for _array_element _outactors
    (if (or (< (Math|Float|Absolute(Float) (- (.x (Transformation|GetActorLocation _array_element)) (.x Location))) (LocalVariables|GetdeltaCoord)) (< (Math|Float|Absolute(Float) (- (.y (Transformation|GetActorLocation _array_element)) (.y Location))) (LocalVariables|GetdeltaCoord)))
      (Utilities|Array|Add (LocalVariables|GetProperTarget) _array_element)))
  (if (> _returnvalue -1)
    (bind _astarget_point (Utilities|Casting|CastToTargetPoint (Utilities|Array|Get(acopy) _propertarget (Math|Random|RandomIntegerinRange 0 (- _returnvalue 1))))
      (:then
        (return _astarget_point true))
      (:CastFailed
        _)))
  (return 0 false))