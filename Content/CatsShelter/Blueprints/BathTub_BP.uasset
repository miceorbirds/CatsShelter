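; An interactable bathtub that cures a cat's fleas in the cat shelter game.
; Interact requires shampoo in the player's inventory and a usable cat item, then consumes the shampoo and clears the cat's flea flag.
; A successful wash raises the water plane via timeline, shows a notification and advances the flea-cure tutorial quest through the game mode.
; Overlap events toggle a custom-depth stencil highlight on the mesh.
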(event Custom|ToggleWater
  (bind _alpha (Timeline|Toggle PlayFromStart)
    (:Update
      (Transformation|SetRelativeLocation (Variables|Default|GetPlane) (Math|Vector|MakeVector 0.0 0.0 (Math|Float|Lerp 1e+01 65.0 _alpha)) false false))))

(event EventBeginPlay)

(event Collision|EventActorBeginOverlap
  (params (OtherActor :type Actor%20Object%20Reference)))

(event EventTick
  (params (DeltaSeconds :type Float%20%28single-precision%29)))

(event EventInteract
  (params (Interactor :type Actor%20Object%20Reference))
  (bind _returnvalue (Game|Player|GetPlayerPawn 0))
  (bind _returnvalue_2 (Actor|GetComponentbyClass _returnvalue "/Game/CatsShelter/InventorySystem/BP_InventoryComponent.BP_InventoryComponent_C"))
  (bind (_isininventory _slotindex) (Default|IsIteminInventory _returnvalue_2 "/Game/CatsShelter/InventorySystem/BP_InventoryItem_Shampoo.BP_InventoryItem_Shampoo_C" 1.0))
  (if _isininventory
    (bind _success (Default|UseItem _returnvalue_2 "/Game/CatsShelter/InventorySystem/BP_InventoryItem_Cat.BP_InventoryItem_Cat_C" 0.0))
    (if _success
      (bind _inventoryslot (Default|DeletefromInventory _returnvalue_2 (Variables|/Game/CatsShelter/InventorySystem/BP_InventoryComponent.BP_InventoryComponent_C|GetCurItem _returnvalue_2) 0.0))
      (Default|DeletefromInventory _returnvalue_2 _slotindex 1.0)
      (Variables|/Game/CatsShelter/Blueprints/Cats/CatInfo.CatInfo_C|SethasFleas (.CatInfo (Utilities|Struct|BreakSInventoryItem (.ItemStructure (Utilities|Struct|BreakSInventorySlot _inventoryslot)))) false)
      (CallFunction|ToggleWater)
      (bind _asthird_person_game_mode (Utilities|Casting|CastToThirdPersonGameMode (Game|GetGameMode)))
      (Default|ShowNotification _asthird_person_game_mode "You have cure the cat!" 1e+01)
      (Default|UpdateQuest _asthird_person_game_mode "/Game/CatsShelter/Quests/Tutorial/BP_Tutorial_CureFleas.BP_Tutorial_CureFleas_C" 1))))

(event EventBeginOverlap
  (bind _staticmeshcomponent (Variables|Debug|GetStaticMeshComponent))
  (Rendering|SetRenderCustomDepth _staticmeshcomponent true)
  (Rendering|SetCustomDepthStencilValue _staticmeshcomponent 2))

(event EventEndOverlap
  (bind _staticmeshcomponent (Variables|Debug|GetStaticMeshComponent))
  (Rendering|SetRenderCustomDepth _staticmeshcomponent false)
  (Rendering|SetCustomDepthStencilValue _staticmeshcomponent 0))

(fn ConstructionScript)