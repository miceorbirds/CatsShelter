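; BP_ComputerDesk is an interactable computer desk in CatsShelter that opens a social network screen for the player.
; Each Interact event toggles the WBP_SocialNetwork widget, creating it on the viewport or removing and clearing it, and also prints a debug message.
; When a ThirdPersonCharacter stops overlapping the Box component, any open widget is closed automatically.
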(event OnComponentEndOverlap(Box)
  (params (OverlappedComponent :type Primitive%20Component%20Object%20Reference) (OtherActor :type Actor%20Object%20Reference) (OtherComp :type Primitive%20Component%20Object%20Reference) (OtherBodyIndex :type Integer))
  (Utilities|Casting|CastToThirdPersonCharacter OtherActor)
  (bind _socialnetwork (Variables|Default|GetSocialNetwork)
    (:then
      (Widget|RemovefromParent _socialnetwork)
      (Variables|Default|SetSocialNetwork 0))
    (:else)))

(event EventInteract
  (params (Interactor :type Actor%20Object%20Reference))
  (Development|PrintString "Hello")
  (bind _socialnetwork (Variables|Default|GetSocialNetwork)
    (:then
      (Widget|RemovefromParent _socialnetwork)
      (Variables|Default|SetSocialNetwork 0))
    (:else
      (bind _returnvalue (UserInterface|CreateWidget "/Game/CatsShelter/UI/SocialNet/WBP_SocialNetwork.WBP_SocialNetwork_C"))
      (bind _output_get (Variables|Default|SetSocialNetwork _returnvalue))
      (UserInterface|Viewport|AddtoViewport _output_get 0))))

(fn ConstructionScript)