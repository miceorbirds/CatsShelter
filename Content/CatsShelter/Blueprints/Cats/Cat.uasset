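; Shelter cat actor that the player can feed, deworm, sterilize, name or pick up as an inventory item, affecting karma and quests.
; A CatInfo object holds its state; timers check it for hunger warnings, death and puddles, and scale the mesh by age.
; Fleas spread to other cats through sphere overlap.
; Player proximity drives a custom-depth highlight and info panel, while interaction plays a meow and opens the action widget.
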(event OnComponentBeginOverlap(Sphere)
  (params (OverlappedComponent :type Primitive%20Component%20Object%20Reference) (OtherActor :type Actor%20Object%20Reference) (OtherComp :type Primitive%20Component%20Object%20Reference) (OtherBodyIndex :type Integer) (bFromSweep :type Boolean) (SweepResult :type Hit%20Result%20Structure%20%28by%20ref%29))
  (if (and (Variables|/Game/CatsShelter/Blueprints/Cats/CatInfo.CatInfo_C|GethasFleas (Variables|Default|GetInfo)) (Actor|ActorHasTag OtherActor "Cat"))
    (bind _ascat (Utilities|Casting|CastToCat OtherActor))
    (CallFunction|SetFleas _ascat)))

(event Custom|CreateWidget
  (params (State :type Integer))
  (Default|ChangeImage (Variables|Default|GetNotice_W) State))

(event Custom|ShowInfoWidget
  (Variables|Default|GetInfo_W
    (:then
      _)
    (:else
      (bind _asthird_person_game_mode (Utilities|Casting|CastToThirdPersonGameMode (Game|GetGameMode)))
      (Variables|Default|SetInfo_W (Variables|/Game/CatsShelter/UI/WBP_MainUI.WBP_MainUI_C|GetWBP_CatInfo (Variables|/Game/CatsShelter/Core/ThirdPersonGameMode.ThirdPersonGameMode_C|GetMainUI _asthird_person_game_mode)))))
  (Widget|SetVisibility (Variables|Default|GetInfo_W) "Visible")
  (Variables|/Game/CatsShelter/UI/WBP_CatInfo.WBP_CatInfo_C|SetInfo (Variables|Default|GetInfo_W) (Variables|Default|GetInfo)))

(event Custom|Initialize
  (params (Info :type Cat%20Info%20Object%20Reference))
  (bind _output_get (Variables|Default|SetInfo Info))
  (CallFunction|UpdateScale)
  (CallFunction|SetColor)
  (Variables|/Game/CatsShelter/Blueprints/Cats/CatInfo.CatInfo_C|SetUrineNeedRate _output_get (* (Variables|/Game/CatsShelter/Blueprints/Cats/CatInfo.CatInfo_C|GetUrineNeedRate _output_get) (Math|Random|RandomFloatinRange 0.8 1.2)))
  (Class|NiagaraComponent|SetPaused (Variables|Default|GetFleas) (not (Variables|/Game/CatsShelter/Blueprints/Cats/CatInfo.CatInfo_C|GethasFleas _output_get)))
  (bind _info_w (Variables|Default|GetInfo_W)
    (:then
      (Variables|/Game/CatsShelter/UI/WBP_CatInfo.WBP_CatInfo_C|SetInfo _info_w (Variables|Default|GetInfo)))
    (:else)))

(event Custom|CheckLiveParams
  (bind _returnvalue (Transformation|GetActorTransform))
  (bind _info (Variables|Default|GetInfo))
  (Utilities|FlowControl|Sequence
    (:then_0
      (if (< (Variables|/Game/CatsShelter/Blueprints/Cats/CatInfo.CatInfo_C|GetSatietyInPercent _info) 3e+01)
        (CallFunction|CreateWidget 2)
        (if (< (Variables|/Game/CatsShelter/Blueprints/Cats/CatInfo.CatInfo_C|GetSatietyInPercent (Variables|Default|GetInfo)) 0.0)
          (bind _asthird_person_game_mode (Utilities|Casting|CastToThirdPersonGameMode (Game|GetGameMode)))
          (Default|ShowNotification _asthird_person_game_mode (Utilities|Text|ToText(String) (Utilities|String|Append (Utilities|String|ToString(Text) (Variables|/Game/CatsShelter/Blueprints/Cats/CatInfo.CatInfo_C|GetName (Variables|Default|GetInfo))) " has dead((((")) 1e+01)
          (bind _asbp_main_game_instance (Utilities|Casting|CastToBP_MainGameInstance (Game|GetGameInstance)))
          (Default|ReduceKarma _asbp_main_game_instance 50)
          (Utilities|Array|RemoveItem (Variables|/Game/CatsShelter/Core/BP_MainGameInstance.BP_MainGameInstance_C|GetCats _asbp_main_game_instance) (Variables|Default|GetInfo))
          (Actor|DestroyActor))))
    (:then_1
      (if (and (> (Variables|/Game/CatsShelter/Blueprints/Cats/CatInfo.CatInfo_C|GetUrineNeedInPercent _info) 1e+02) (not (Variables|Default|GetFreeToMove)))
        (Game|SpawnActorfromClass "/Game/CatsShelter/Blueprints/Cats/Puddle.Puddle_C" (Math|Transform|MakeTransform (Math|Vector|MakeVector (.x (.location _returnvalue)) (.y (.location _returnvalue)) (- (.z (.location _returnvalue)) 1e+01)) (.rotation _returnvalue) "1,1,1") "Undefined" 0 0)
        (Variables|/Game/CatsShelter/Blueprints/Cats/CatInfo.CatInfo_C|SetUrineNeedInPercent (Variables|Default|GetInfo) 0.0)
        (Variables|Default|SetFreeToMove false)
        (AI|Navigation|StopMovement (Pawn|GetController))
        (Animation|Montage|PlayMontage (Variables|Character|GetMesh) "/Game/CatsShelter/Core/Cat/AM_Cat_Poo.AM_Cat_Poo"
          (:OnCompleted
            _)
          (:OnInterrupted
            _))
        (Variables|Default|SetFreeToMove true)
        (Default|CallPlayerWalkedAway)))
    (:then_2
      (if (and (Class|NiagaraComponent|IsPaused (Variables|Default|GetFleas)) (Variables|/Game/CatsShelter/Blueprints/Cats/CatInfo.CatInfo_C|GethasFleas (Variables|Default|GetInfo)))
        (Class|NiagaraComponent|SetPaused (Variables|Default|GetFleas) false)))))

(event Custom|HideInfoWidget
  (Widget|SetVisibility (Variables|Default|GetInfo_W) "Hidden"))

(event Custom|Eat
  (bind _returnvalue (Game|Player|GetPlayerPawn 0))
  (bind _info (Variables|Default|GetInfo))
  (bind _returnvalue_2 (Actor|GetComponentbyClass _returnvalue "/Game/CatsShelter/InventorySystem/BP_InventoryComponent.BP_InventoryComponent_C"))
  (bind _curitem (Variables|/Game/CatsShelter/InventorySystem/BP_InventoryComponent.BP_InventoryComponent_C|GetCurItem _returnvalue_2))
  (bind _list_of_slots (Variables|/Game/CatsShelter/InventorySystem/BP_InventoryComponent.BP_InventoryComponent_C|GetList%20of%20Slots _returnvalue_2))
  (bind _output (Utilities|Array|Get(acopy) _list_of_slots _curitem))
  (bind _itemstructure (Utilities|Struct|BreakSInventorySlot _output))
  (bind (_itemname _itemthumbnail _isstackable _maxstacksize _portions _class) (Utilities|Struct|BreakSInventoryItem _itemstructure))
  ;[1 1 1] Feed the cat
  (Variables|Default|GetInfo
    (:then
      (switch string (Utilities|String|ToString(Text) _itemname)
        (:Cat%20Food
          ;;[1 1 1] Check whether cat is full or not
          (if (== (Variables|/Game/CatsShelter/Blueprints/Cats/CatInfo.CatInfo_C|GetSatietyInPercent (Variables|Default|GetInfo)) 1e+02) :!label _label
            ;;[1 1 1] Have the player the item in inventory?
            (bind _asthird_person_game_mode (Utilities|Casting|CastToThirdPersonGameMode (Game|GetGameMode)))
            (Default|ShowNotification _asthird_person_game_mode "Cat is full." 1e+01)
            (else
              (bind _success (Default|UseItem (Actor|GetComponentbyClass (Game|Player|GetPlayerPawn 0) "/Game/CatsShelter/InventorySystem/BP_InventoryComponent.BP_InventoryComponent_C") _class (Variables|Default|GetAmountOfFood)))
              (if _success
                (bind _output_get (Variables|/Game/CatsShelter/Blueprints/Cats/CatInfo.CatInfo_C|SetSatietyInPercent (Variables|Default|GetInfo) (+ (Variables|/Game/CatsShelter/Blueprints/Cats/CatInfo.CatInfo_C|GetSatietyInPercent (Variables|Default|GetInfo)) 5e+01)))
                (if (> _output_get 1e+02)
                  (Variables|/Game/CatsShelter/Blueprints/Cats/CatInfo.CatInfo_C|SetSatietyInPercent (Variables|Default|GetInfo) 1e+02))
                (bind _asthird_person_game_mode_2 (Utilities|Casting|CastToThirdPersonGameMode (Game|GetGameMode)))
                (Default|UpdateQuest _asthird_person_game_mode_2 "/Game/CatsShelter/Quests/BP_Quest_Feed.BP_Quest_Feed_C" 1)
                (Default|UpdateQuest _asthird_person_game_mode_2 "/Game/CatsShelter/Quests/Tutorial/BP_Tutorial_Feed.BP_Tutorial_Feed_C" 1)
                (CallFunction|CreateWidget 1 :!label _label_2)
                (Utilities|FlowControl|Delay 3.0)
                (CallFunction|CreateWidget)
                (bind _asbp_main_game_instance (Utilities|Casting|CastToBP_MainGameInstance (Game|GetGameInstance)))
                (Default|IncreaseKarma _asbp_main_game_instance (Variables|Default|GetAddedKarma))
                (else
                  (bind _asthird_person_game_mode_3 (Utilities|Casting|CastToThirdPersonGameMode (Game|GetGameMode)))
                  (Default|ShowNotification _asthird_person_game_mode_3 "Not enough food." 1e+01))))))
        (:Cat%20Food%20Premium
          (goto _label))
        (:Antiwormer
          (bind _success_2 (Default|UseItem (Actor|GetComponentbyClass (Game|Player|GetPlayerPawn 0) "/Game/CatsShelter/InventorySystem/BP_InventoryComponent.BP_InventoryComponent_C") _class 1.0))
          (if _success_2
            (Variables|/Game/CatsShelter/Blueprints/Cats/CatInfo.CatInfo_C|SethasWorms _info false)
            (Variables|/Game/CatsShelter/Blueprints/Cats/CatInfo.CatInfo_C|SetHungerRate _info 0.2)
            (bind _asthird_person_game_mode_4 (Utilities|Casting|CastToThirdPersonGameMode (Game|GetGameMode)))
            (Default|UpdateQuest _asthird_person_game_mode_4 "/Game/CatsShelter/Quests/Tutorial/BP_Tutorial_CureWorms.BP_Tutorial_CureWorms_C" 1)
            (goto _label_2)))))
    (:else)))

(event Custom|Sterilize
  (bind _info (Variables|Default|GetInfo)
    (:then
      (if (not (Variables|/Game/CatsShelter/Blueprints/Cats/CatInfo.CatInfo_C|GetisSterilized _info))
        (Variables|/Game/CatsShelter/Blueprints/Cats/CatInfo.CatInfo_C|SetisSterilized _info true)
        (bind _asthird_person_game_mode (Utilities|Casting|CastToThirdPersonGameMode (Game|GetGameMode)))
        (Default|UpdateQuest _asthird_person_game_mode "/Game/CatsShelter/Quests/Tutorial/BP_Tutorial_Sterilize.BP_Tutorial_Sterilize_C" 1)
        (bind _asbp_main_game_instance (Utilities|Casting|CastToBP_MainGameInstance (Game|GetGameInstance)))
        (Default|IncreaseKarma _asbp_main_game_instance (Variables|Default|GetAddedKarma))
        (else
          (bind _asthird_person_game_mode_2 (Utilities|Casting|CastToThirdPersonGameMode (Game|GetGameMode)))
          (Default|ShowNotification _asthird_person_game_mode_2 "Cat already sterilized!" 1e+01))))
    (:else)))

(event Custom|GiveName
  (bind _info (Variables|Default|GetInfo)
    (:then
      (bind _aspc_configurator (Utilities|Casting|CastToPC_Configurator (Game|GetPlayerController 0)))
      (Variables|/Game/CatsShelter/UI/WBP_TextInput.WBP_TextInput_C|SetCat (Variables|/Game/CatsShelter/UI/WBP_HUD.WBP_HUD_C|GetWBP_TextInput (Variables|/Game/CatsShelter/Core/PC_Configurator.PC_Configurator_C|GetMain%20HUD%20widget _aspc_configurator)) _info)
      (Input|SetInputModeUIOnly _aspc_configurator (Variables|/Game/CatsShelter/UI/WBP_TextInput.WBP_TextInput_C|GetEditableTextBox_59 (Variables|/Game/CatsShelter/UI/WBP_HUD.WBP_HUD_C|GetWBP_TextInput (Variables|/Game/CatsShelter/Core/PC_Configurator.PC_Configurator_C|GetMain%20HUD%20widget _aspc_configurator))) "DoNotLock")
      (Widget|SetVisibility (Variables|/Game/CatsShelter/UI/WBP_HUD.WBP_HUD_C|GetWBP_TextInput (Variables|/Game/CatsShelter/Core/PC_Configurator.PC_Configurator_C|GetMain%20HUD%20widget _aspc_configurator)) "Visible")
      (Widget|SetKeyboardFocus (Variables|/Game/CatsShelter/UI/WBP_TextInput.WBP_TextInput_C|GetEditableTextBox_59 (Variables|/Game/CatsShelter/UI/WBP_HUD.WBP_HUD_C|GetWBP_TextInput (Variables|/Game/CatsShelter/Core/PC_Configurator.PC_Configurator_C|GetMain%20HUD%20widget _aspc_configurator))))
      (bind _asbp_main_game_instance (Utilities|Casting|CastToBP_MainGameInstance (Game|GetGameInstance)))
      (Default|IncreaseKarma _asbp_main_game_instance (Variables|Default|GetAddedKarma)))
    (:else)))

(event Custom|SetFleas
  (bind _info (Variables|Default|GetInfo))
  (if (not (Variables|/Game/CatsShelter/Blueprints/Cats/CatInfo.CatInfo_C|GethasFleas _info))
    (Variables|/Game/CatsShelter/Blueprints/Cats/CatInfo.CatInfo_C|SethasFleas _info true)
    (Class|NiagaraComponent|SetPaused (Variables|Default|GetFleas) false)
    (bind _asbp_main_game_instance (Utilities|Casting|CastToBP_MainGameInstance (Game|GetGameInstance)))
    (Default|ReduceKarma _asbp_main_game_instance (Variables|Default|GetAddedKarma))))

(event Custom|Take
  (bind _result (CallFunction|IsHomeless (Variables|Default|GetInfo)))
  (if _result
    (bind _asbp_main_game_instance (Utilities|Casting|CastToBP_MainGameInstance (Game|GetGameInstance)))
    (bind _catinfo (Default|CreateCatInfo _asbp_main_game_instance))
    (bind _output_get (Variables|Default|SetInfo _catinfo))
    (Variables|/Game/CatsShelter/Blueprints/Cats/CatInfo.CatInfo_C|SethasFleas _output_get true)
    (Variables|/Game/CatsShelter/Blueprints/Cats/CatInfo.CatInfo_C|SethasWorms _output_get true)
    (bind _asthird_person_game_mode (Utilities|Casting|CastToThirdPersonGameMode (Game|GetGameMode)))
    (Default|UpdateQuest _asthird_person_game_mode "/Game/CatsShelter/Quests/Tutorial/BP_Tutorial_Take.BP_Tutorial_Take_C" 1)
    (bind _asbp_main_game_instance_2 (Utilities|Casting|CastToBP_MainGameInstance (Game|GetGameInstance)))
    (Default|IncreaseKarma _asbp_main_game_instance_2 (Variables|Default|GetAddedKarma)))
  (bind _output_get_2 (Variables|/Game/CatsShelter/Blueprints/Cats/CatInfo.CatInfo_C|SetInventoryItemStruct (Variables|Default|GetInfo) (Utilities|Struct|MakeSInventoryItem (Variables|/Game/CatsShelter/Blueprints/Cats/CatInfo.CatInfo_C|GetName (Variables|Default|GetInfo)) "/Game/CatsShelter/Blueprints/Widgets/smilingCat.smilingCat" false 1 1.0 "/Game/CatsShelter/InventorySystem/BP_InventoryItem_Cat.BP_InventoryItem_Cat_C" (Variables|Default|GetInfo) 0 "")))
  (bind _succeed (Default|AddItemtoInventory (Actor|GetComponentbyClass (Game|Player|GetPlayerPawn 0) "/Game/CatsShelter/InventorySystem/BP_InventoryComponent.BP_InventoryComponent_C") _output_get_2))
  (if _succeed
    (CallFunction|HideInfoWidget)
    (Actor|DestroyActor)))

(event EventBeginPlay
  (Utilities|Time|SetTimerbyFunctionName 0 "UpdateScale" 1e+01 true)
  (Utilities|Time|SetTimerbyEvent (delegate Custom|CheckLiveParams) 1.0 true)
  (bind _ascat_notice_widget (Utilities|Casting|CastToCatNoticeWidget (UserInterface|GetUserWidgetObject (Variables|Default|GetWidget))))
  (bind _output_get (Variables|Default|SetNotice_W _ascat_notice_widget))
  (Variables|/Game/CatsShelter/UI/WBP_Interaction.WBP_Interaction_C|SetCat (Variables|/Game/CatsShelter/Blueprints/Widgets/CatNoticeWidget.CatNoticeWidget_C|GetWBP_Interaction _output_get) self)
  (Widget|SetVisibility (Variables|/Game/CatsShelter/Blueprints/Widgets/CatNoticeWidget.CatNoticeWidget_C|GetWBP_Interaction _output_get) "Hidden"))

(event EventInteract
  (params (Interactor :type Actor%20Object%20Reference))
  (bind _catmews (Variables|Default|GetCatMews))
  (Widget|SetVisibility (Variables|/Game/CatsShelter/Blueprints/Widgets/CatNoticeWidget.CatNoticeWidget_C|GetWBP_Interaction (Variables|Default|GetNotice_W)) "Visible")
  (Audio|SpawnSoundatLocation (Utilities|Array|Get(acopy) _catmews (Math|Random|RandomIntegerinRange 0 (- (Utilities|Array|Length _catmews) 1))) (Transformation|GetWorldLocation (Variables|Character|GetMesh)) "0, 0, 0" 1.0 1.0 0.0 0 0))

(event EventBeginOverlap
  (bind _mesh (Variables|Character|GetMesh))
  (Default|CallPlayerWalkedNearby)
  (Rendering|SetRenderCustomDepth _mesh true)
  (Rendering|SetCustomDepthStencilValue _mesh 2)
  (CallFunction|ShowInfoWidget))

(event EventEndOverlap
  (bind _mesh (Variables|Character|GetMesh))
  (Rendering|SetRenderCustomDepth _mesh false)
  (Rendering|SetCustomDepthStencilValue _mesh 0)
  (CallFunction|HideInfoWidget)
  (Widget|SetVisibility (Variables|/Game/CatsShelter/Blueprints/Widgets/CatNoticeWidget.CatNoticeWidget_C|GetWBP_Interaction (Variables|Default|GetNotice_W)) "Hidden")
  (Default|CallPlayerWalkedAway)
  (Animation|StopAnimMontage "/Game/CatsShelter/Core/Cat/AM_Cat_Poo.AM_Cat_Poo"))

(fn ConstructionScript
  (bind _returnvalue (Game|ConstructObjectfromClass "/Game/CatsShelter/Blueprints/Cats/CatInfo.CatInfo_C" self))
  (Variables|Default|SetInfo _returnvalue)
  (Class|NiagaraComponent|SetPaused (Variables|Default|GetFleas) true))

(fn IsHomeless
  (params (CatInfo :type Cat%20Info%20Object%20Reference))
  (bind _asbp_main_game_instance (Utilities|Casting|CastToBP_MainGameInstance (Game|GetGameInstance)))
  (for _array_element (Variables|/Game/CatsShelter/Core/BP_MainGameInstance.BP_MainGameInstance_C|GetCats _asbp_main_game_instance)
    (if (== _array_element CatInfo)
      (return false)))
  (return true))

(fn UpdateScale
  (bind _info (Variables|Default|GetInfo))
  (bind _age (Variables|/Game/CatsShelter/Blueprints/Cats/CatInfo.CatInfo_C|GetAge _info))
  (bind _asthird_person_game_mode (Utilities|Casting|CastToThirdPersonGameMode (Game|GetGameMode)))
  (if (< _age (Variables|/Game/CatsShelter/Core/ThirdPersonGameMode.ThirdPersonGameMode_C|GetminAgeForPregnancy _asthird_person_game_mode))
    (Transformation|SetActorScale3D (Math|Vector|MakeVector (+ (/ (* _age 0.6) (Math|Conversions|ToFloat(Integer) (Variables|/Game/CatsShelter/Core/ThirdPersonGameMode.ThirdPersonGameMode_C|GetminAgeForPregnancy _asthird_person_game_mode))) 0.4) (+ (/ (* _age 0.6) (Math|Conversions|ToFloat(Integer) (Variables|/Game/CatsShelter/Core/ThirdPersonGameMode.ThirdPersonGameMode_C|GetminAgeForPregnancy _asthird_person_game_mode))) 0.4) (+ (/ (* _age 0.6) (Math|Conversions|ToFloat(Integer) (Variables|/Game/CatsShelter/Core/ThirdPersonGameMode.ThirdPersonGameMode_C|GetminAgeForPregnancy _asthird_person_game_mode))) 0.4)))
    (else
      (Transformation|SetActorScale3D (Math|Vector|MakeVector 1.0 1.0 1.0)))))

(fn SetColor
  (bind _info (Variables|Default|GetInfo)
    (:then
      (Rendering|Material|SetMaterial (Variables|Character|GetMesh) 0 (Variables|/Game/CatsShelter/Blueprints/Cats/CatInfo.CatInfo_C|GetColor _info)))
    (:else)))