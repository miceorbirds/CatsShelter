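; AI controller for shelter cats that wander at random and react when the player comes near.
; A looping timer with random start variance sends the cat to a reachable NavMesh point, choosing the next destination once each move finishes.
; The cat's nearby event pauses wandering, moves it toward the player and turns its yaw with a LookAt timeline.
; The walked-away event restores free movement and resumes wandering.
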(event Custom|PlayerWalkedNearby_Event_0
  (bind _controlledcat (Variables|Default|GetControlledCat))
  (bind _returnvalue (Transformation|GetActorRotation _controlledcat))
  (bind (_roll _pitch) (Math|Rotator|BreakRotator _returnvalue))
  (Variables|/Game/CatsShelter/Blueprints/Cats/Cat.Cat_C|SetFreeToMove (Variables|Default|GetControlledCat) false)
  (AI|Navigation|MovetoActor (Game|Player|GetPlayerPawn 0) 1.5e+02 true true true 0)
  (bind _alpha (Timeline|LookAt PlayFromStart)
    (:Update
      (Transformation|SetActorRotation _controlledcat (Math|Rotator|MakeRotator _roll _pitch (.yaw (Math|Rotator|Lerp(Rotator) _returnvalue (Math|Rotator|FindLookatRotation (Transformation|GetActorLocation _controlledcat) (Transformation|GetActorLocation (Game|GetPlayerCharacter 0))) _alpha true)))))))

(event Custom|MoveToRandomPoint
  (if (Variables|/Game/CatsShelter/Blueprints/Cats/Cat.Cat_C|GetFreeToMove (Variables|Default|GetControlledCat))
    (AI|AIMoveTo (Pawn|GetControlledPawn) (Variables|Default|GetDestination) 0 5e+01 false
      (:OnSuccess
        _)
      (:OnFail
        _))
    (Variables|Default|SetDestination (.RandomLocation (AI|Navigation|GetRandomReachablePointinRadius (Transformation|GetActorLocation (Pawn|GetControlledPawn)) 1e+03 0 0)))))

(event Custom|PlayerWalkedAway_Event_0
  (Variables|/Game/CatsShelter/Blueprints/Cats/Cat.Cat_C|SetFreeToMove (Variables|Default|GetControlledCat) true)
  (CallFunction|MovetoRandomPoint))

(event EventBeginPlay
  (Utilities|FlowControl|Delay 0.2)
  (bind _ascat (Utilities|Casting|CastToCat (Pawn|GetControlledPawn)))
  (bind _output_get (Variables|Default|SetControlledCat _ascat))
  (Variables|Default|SetDestination (.RandomLocation (AI|Navigation|GetRandomReachablePointinRadius (Transformation|GetActorLocation _output_get) 1e+03 0 0)))
  (CallFunction|MovetoRandomPoint)
  (Utilities|Time|SetTimerbyEvent (delegate Custom|MoveToRandomPoint) 2e+01 true 0.0 1e+01)
  (EventDispatchers|AssignPlayerWalkedNearby (Variables|Default|GetControlledCat) (delegate Custom|PlayerWalkedNearby_Event_0))
  (EventDispatchers|AssignPlayerWalkedAway (Variables|Default|GetControlledCat) (delegate Custom|PlayerWalkedAway_Event_0)))

(fn ConstructionScript)