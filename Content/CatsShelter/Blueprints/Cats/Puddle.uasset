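; Puddle actor in the cat shelter game that appears by growing and is removed when interacted with.
; On BeginPlay a timeline scales it up from near zero to a small final size.
; BeginOverlap and EndOverlap events toggle custom depth and a stencil value on its mesh, marking it for a highlight, and Interact destroys the actor.
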(event EventBeginPlay
  (bind _newtrack_0 (Timeline|Timeline_0 PlayFromStart)
    (:Update
      (Transformation|SetActorScale3D (Math|Vector|Lerp(Vector) "0.010000,0.010000,0.010000" "0.100000,0.100000,0.100000" _newtrack_0)))))

(event Collision|EventActorBeginOverlap
  (params (OtherActor :type Actor%20Object%20Reference)))

(event EventTick
  (params (DeltaSeconds :type Float%20%28single-precision%29)))

(event EventInteract
  (params (Interactor :type Actor%20Object%20Reference))
  (Actor|DestroyActor))

(event EventBeginOverlap
  (bind _staticmeshcomponent (Variables|Debug|GetStaticMeshComponent))
  (Rendering|SetRenderCustomDepth _staticmeshcomponent true)
  (Rendering|SetCustomDepthStencilValue _staticmeshcomponent 2))

(event EventEndOverlap
  (bind _staticmeshcomponent (Variables|Debug|GetStaticMeshComponent))
  (Rendering|SetRenderCustomDepth _staticmeshcomponent false)
  (Rendering|SetCustomDepthStencilValue _staticmeshcomponent 0))

(fn ConstructionScript)